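; VR movement component that flies its owning Character relative to a supplied camera.
; Setup caches camera and Character and switches movement to Flying.
; Move functions feed camera-forward, flattened camera-right or actor-up movement input, while FlyUp and Yawing offset the actor directly, all with slower variants.
; Tick remaps DistanceToGround, never updated here, into max fly speed and braking, a workaround the author notes keeps movement working.
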(event `self.ReceiveTick`
  (params (DeltaSeconds :type "Float (single-precision)"))
  (`parent.ReceiveTick` DeltaSeconds)
  (`self.SetMaxSpeed`))

(fn `FlyUp`
  (params (InputValue :type "Float (double-precision)"))
  (`Actor.K2_AddActorLocalTransform` (`self._character`) (`KismetMathLibrary.MakeTransform` (`KismetMathLibrary.MakeVector` 0.0 0.0 (* InputValue 6.0))) false false))

(fn `Move Left`
  (params (inputValue :type "Float (double-precision)"))
  (`Pawn.AddMovementInput` (`self._character`) (`KismetMathLibrary.MakeVector` (.x (`SceneComponent.GetRightVector` (`self._cameraComponent`))) (.y (`SceneComponent.GetRightVector` (`self._cameraComponent`)))) (* inputValue 0.3) false)
  (return))

(fn `MoveForward`
  (params (inputValue :type "Float (double-precision)"))
  (`Pawn.AddMovementInput` (`self._character`) (`SceneComponent.GetForwardVector` (`self._cameraComponent`)) (* inputValue 0.3) false)
  (return))

(fn `MoveUp`
  (params (inputValue :type "Float (double-precision)"))
  (`Pawn.AddMovementInput` (`self._character`) (`Actor.GetActorUpVector` (`self._character`)) (* inputValue 0.5) false)
  (return))

(fn `SetMaxSpeed`
  (bind _charactermovement (`Character.CharacterMovement` (`self._character`)))
  ;[0.6667 0.444 0.02024 1 14] We don't use these valuables, but refering project has this function. If I don't call this function every tick, movement interaction doesn't work well.
  ; If you have any tips to fix movement system without this function, I would be glad you to report it to me
  (bind _output_get (set `CharacterMovementComponent.MaxFlySpeed` (`KismetMathLibrary.MapRangeClamped` (`self.DistanceToGround`) (`self.GroundSnapDistance`) (`self.MaxSpeedAltitude`) 1500.0 (`self.MaxFlySpeed`)) _charactermovement))
  (set `CharacterMovementComponent.BrakingDecelerationFlying` (* _output_get 5.0) _charactermovement)
  (return))

(fn `Setup`
  (params (cameraComponent :type "CameraComponent Object Reference (by ref)") (Foot_Z_Offset :type "Float (double-precision)"))
  (set `self._cameraComponent` cameraComponent)
  (set `self.FootZOffset` Foot_Z_Offset)
  (bind _ascharacter (cast `Character` (`self.GetOwner`)))
  (bind _output_get (set `self._character` _ascharacter))
  (`CharacterMovementComponent.SetMovementMode` (`Character.CharacterMovement` _output_get) "MOVE_Flying" 0)
  (return))

(fn `SlowFlyUp`
  (params (InputValue :type "Float (double-precision)"))
  (`Actor.K2_AddActorLocalTransform` (`self._character`) (`KismetMathLibrary.MakeTransform` (`KismetMathLibrary.MakeVector` 0.0 0.0 (* InputValue 1.0))) false false))

(fn `SlowMoveForward`
  (params (inputValue :type "Float (double-precision)"))
  (`Pawn.AddMovementInput` (`self._character`) (`SceneComponent.GetForwardVector` (`self._cameraComponent`)) (* inputValue 0.05) false))

(fn `SlowMoveLeft`
  (params (inputValue :type "Float (double-precision)"))
  (`Pawn.AddMovementInput` (`self._character`) (`KismetMathLibrary.MakeVector` (.x (`SceneComponent.GetRightVector` (`self._cameraComponent`))) (.y (`SceneComponent.GetRightVector` (`self._cameraComponent`)))) (* inputValue 0.1) false)
  (return))

(fn `SlowMoveUp`
  (params (inputValue :type "Float (double-precision)"))
  (`Pawn.AddMovementInput` (`self._character`) (`Actor.GetActorUpVector` (`self._character`)) (* inputValue 0.2) false)
  (return))

(fn `SlowYawing`
  (params (InputValue :type "Float (double-precision)"))
  (`Actor.K2_AddActorLocalRotation` (`self._character`) (`KismetMathLibrary.MakeRotator` 0.0 0.0 (* InputValue 0.3)) false false))

(fn `Yawing`
  (params (InputValue :type "Float (double-precision)"))
  (`Actor.K2_AddActorLocalRotation` (`self._character`) (`KismetMathLibrary.MakeRotator` 0.0 0.0 (* InputValue 1.5)) false false))